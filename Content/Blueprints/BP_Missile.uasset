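; BP_Missile is a short-lived missile actor that destroys actors tagged Target on overlap.
; On a hit it removes the target, plays an explosion sound, spawns an emitter, then calls CheckStage on the BP_GM game mode before destroying itself.
; A missile that hits nothing destroys itself after a fixed delay from BeginPlay.
; The graphs contain no movement logic, and Tick is unused.
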(event `self.ReceiveBeginPlay`
  (`KismetSystemLibrary.Delay` 3.0)
  (`self.K2_DestroyActor`))

(event `self.ReceiveActorBeginOverlap`
  (params (OtherActor :type "Actor Object Reference"))
  (if (`self.ActorHasTag` OtherActor "Target")
    (`self.K2_DestroyActor` OtherActor)
    (`GameplayStatics.SpawnSoundAtLocation` "/Game/StarterContent/Audio/Explosion_Cue.Explosion_Cue" (`self.K2_GetActorLocation`) (struct) 1.0 1.0 0.0 null null)
    (`GameplayStatics.SpawnEmitterAtLocation` null (`self.K2_GetActorLocation`))
    (bind _asbp_gm (cast `/Game/Blueprints/BP_GM` (`GameplayStatics.GetGameMode`)))
    (`/Game/Blueprints/BP_GM.CheckStage` _asbp_gm)
    (`self.K2_DestroyActor`)))

(fn `UserConstructionScript`)